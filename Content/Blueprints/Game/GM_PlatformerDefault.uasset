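; GM_PlatformerDefault is a platformer game mode that tracks how many enemies remain to decide when the level is won.
; EncreaseEnemy and DecreaseEnemy adjust the Enemes counter, and a decrease to zero or below calls WinGame.
; WinGame is an empty event in this graph, and Tick prints the current count on screen every frame as a debug readout.
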(event Custom|EncreaseEnemy
  (Math|Integer|IncrementInt (Variables|Default|GetEnemes)))

(event Custom|DecreaseEnemy
  (bind _result (Math|Integer|DecrementInt (Variables|Default|GetEnemes))
    (:%20%20
      (if (<= _result 0)
        (CallFunction|WinGame)))))

(event Custom|WinGame)

(event EventTick
  (params (DeltaSeconds :type Float%20%28single-precision%29))
  (Development|PrintString (Utilities|String|ToString(Integer) (Variables|Default|GetEnemes)) true true "(R=0.000000,G=0.660000,B=1.000000,A=1.000000)" 0.0))

(fn ConstructionScript)