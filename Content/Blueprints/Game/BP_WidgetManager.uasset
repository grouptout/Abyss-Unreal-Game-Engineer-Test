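; BP_WidgetManager creates and updates the on-screen enemies-remaining counter for the platformer game mode.
; On BeginPlay it binds to the EnemiesChanged dispatcher on GM_PlatformerDefault, adds a W_EnemiesRemaining widget to the viewport and triggers an initial refresh.
; Its event handler passes the game mode's Enemies value to the widget's ChangeEnemyText, so the display is event-driven without polling.
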(event Custom|EnemiesChanged_Event
  (Default|ChangeEnemyText (Variables|Default|GetEnemyWidget) (Variables|/Game/Blueprints/Game/GM_PlatformerDefault.GM_PlatformerDefault_C|GetEnemies (.AsGM%20Platformer%20Default (Utilities|Casting|CastToGM_PlatformerDefault (Game|GetGameMode))))))

(event EventBeginPlay
  (EventDispatchers|AssignEnemiesChanged (.AsGM%20Platformer%20Default (Utilities|Casting|CastToGM_PlatformerDefault (Game|GetGameMode))) (delegate Custom|EnemiesChanged_Event))
  (bind _returnvalue (UserInterface|CreateWidget "/Game/UI/W_EnemiesRemaining.W_EnemiesRemaining_C"))
  (UserInterface|Viewport|AddtoViewport _returnvalue 0)
  (Variables|Default|SetEnemyWidget _returnvalue)
  (CallFunction|EnemiesChangedEvent))

(fn ConstructionScript)