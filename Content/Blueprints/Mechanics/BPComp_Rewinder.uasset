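; Actor component that gives its owner time rewind, toggled by TimeRewinding and TimeNormalizing events.
; Each Tick either records location or transform, plus optional skeletal mesh velocities and anim poses, or pops those stacks to play history backwards.
; Linear and angular velocities share one Transform as Location and Scale; poses pass through AnimInstance messages.
; Arrays drop their oldest half at a critical count to bound memory.
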(event EventBeginPlay)

(event EventTick
  (params (DeltaSeconds :type Float%20%28single-precision%29))
  (if (Variables|Default|GetRewinding?)
    (CallFunction|ProcessRewinding)
    (else
      (CallFunction|RecordforRewinding))))

(event EventTimeNormalizing
  (Variables|Default|SetRewinding? false))

(event EventTimeRewinding
  (Variables|Default|SetRewinding? true))

(fn ProcessRewinding
  (Utilities|FlowControl|Sequence
    (:then_0
      ;[1 1 1 0.091] Locations or transforms
      (switch Utilities|FlowControl|Switch|SwitchonE_RewindMode (Variables|RewindMode|GetRewindMode)
        (:NewEnumerator0
          (if (> (Utilities|Array|LastIndex (Variables|Default|GetActorLocationsOnly)) 0)
            (|ControlLocations :!label _label)
            (else
              (goto _label False))))
        (:NewEnumerator1
          (if (> (Utilities|Array|LastIndex (Variables|Default|GetActorTransforms)) 0)
            (|ControlTransforms_2 :!label _label_2)
            (else
              (goto _label_2 Last))))))
    (:then_1
      ;[1 1 1 0.091] Physics
      (if (Variables|RewindMode|GetRewindPhysics?)
        (|ControlPhys)))
    (:then_2
      ;[1 1 1 0.089] Animations
      (if (Variables|RewindMode|GetRewindAnims?)
        (|AnimationControl)))))

(fn RecordforRewinding
  (bind _returnvalue (Components|GetOwner))
  (bind _returnvalue_2 (Components|GetOwner))
  (bind _criticalcountoptimization (Variables|Default|GetCriticalCountOptimization))
  (bind _actortransforms (Variables|Default|GetActorTransforms))
  (bind _actorvelocities (Variables|Default|GetActorVelocities))
  (bind _snapshot (Variables|Default|GetSnapshot))
  (bind _actorlocationsonly (Variables|Default|GetActorLocationsOnly))
  (bind _returnvalue_3 (Actor|GetComponentbyClass _returnvalue "/Script/Engine.SkeletalMeshComponent"))
  (bind _returnvalue_4 (Actor|GetComponentbyClass _returnvalue_2 "/Script/Engine.SkeletalMeshComponent"))
  (bind _returnvalue_5 (Components|SkeletalMesh|GetAnimInstance _returnvalue_4))
  (Utilities|FlowControl|Sequence
    (:then_0
      (switch Utilities|FlowControl|Switch|SwitchonE_RewindMode (Variables|RewindMode|GetRewindMode)
        (:NewEnumerator0
          ;[1 1 1 0.079] Record locations or transforms
          (Utilities|Array|Add _actorlocationsonly (Transformation|GetActorLocation (Components|GetOwner)))
          ;[0.08843 0 1 0.154] Memory half-cleaner
          (Utilities|ClearTArray _actorlocationsonly _criticalcountoptimization))
        (:NewEnumerator1
          (Utilities|Array|Add _actortransforms (Transformation|GetActorTransform (Components|GetOwner)))
          (Utilities|ClearTArray _actortransforms _criticalcountoptimization))))
    (:then_1
      ;[1 1 1 0.068] Record velocity
      (if (Variables|RewindMode|GetRewindPhysics?)
        (bind _returnvalue_6 (Physics|GetPhysicsLinearVelocity _returnvalue_3 "None"))
        (Utilities|Array|Add _actorvelocities (Math|Transform|MakeTransform _returnvalue_6 "0, 0, 0" (Physics|GetPhysicsAngularVelocityinDegrees _returnvalue_3 "None")))
        (Utilities|ClearTArray _actorvelocities _criticalcountoptimization)))
    (:then_2
      ;[1 1 1 0.029] Record animations
      (if (Variables|RewindMode|GetRewindAnims?)
        (bind _pose (Class|BPIAnimRewindable|GetPose(Message) _returnvalue_5))
        (Utilities|Array|Add _snapshot _pose)
        (Class|BPIAnimRewindable|SetIsRewinding(Message) _returnvalue_5 false)
        (Utilities|ClearTArray _snapshot _criticalcountoptimization)))))