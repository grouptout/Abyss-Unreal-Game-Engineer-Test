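; Character Blueprint that records its movement every tick and plays it backwards while time rewind is active.
; RewindTime and NormalizeTime toggle the mode; normal ticks append transforms and physics velocities to uncapped arrays, packing linear and angular velocity into a transform's location and scale.
; Rewinding ticks apply and pop the newest transform, holding at the oldest.
; Velocity playback applies the first recorded entry while trimming from the end.
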(event EventTick
  (params (DeltaSeconds :type Float%20%28single-precision%29))
  (if (Variables|Default|GetRewinding?)
    (CallFunction|ProcessRewinding)
    (else
      (CallFunction|RecordforRewinding))))

(event EventRewindTime
  (Variables|Default|SetRewinding? true))

(event EventNormalizeTime
  (Variables|Default|SetRewinding? false))

(fn ConstructionScript)

(fn ProcessRewinding
  (Utilities|FlowControl|Sequence
    (:then_0
      (if (> (Utilities|Array|LastIndex (Variables|Default|GetActorTransforms)) 0)
        (|ControlTransforms :!label _label)
        (else
          (goto _label Last))))
    (:then_1
      (if (> (Utilities|Array|LastIndex (Variables|Default|GetActorVelocities)) 0)
        (|ControlVelocities)))))

(fn RecordforRewinding
  (bind _charactermovement (Variables|Character|GetCharacterMovement))
  (bind _updatedprimitive (Variables|/Script/Engine.MovementComponent|GetUpdatedPrimitive _charactermovement))
  (Utilities|FlowControl|Sequence
    (:then_0
      ;[1 1 1 0.079] Record transforms
      (Utilities|Array|Add (Variables|Default|GetActorTransforms) (Transformation|GetActorTransform self)))
    (:then_1
      ;[1 1 1 0.079] Record velocities
      (bind _returnvalue (Physics|GetPhysicsLinearVelocity _updatedprimitive "None"))
      (Utilities|Array|Add (Variables|Default|GetActorVelocities) (Math|Transform|MakeTransform _returnvalue "0, 0, 0" (Physics|GetPhysicsAngularVelocityinDegrees _updatedprimitive "None"))))))