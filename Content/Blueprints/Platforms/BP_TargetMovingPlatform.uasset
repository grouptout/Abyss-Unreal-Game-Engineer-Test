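; BP_TargetMovingPlatform is a platform that shuttles back and forth between its placed position and a target location.
; On BeginPlay it converts TargetLocation from actor-local to world space and caches the journey length.
; Each tick it swaps start and target once the distance travelled reaches that length.
; It then moves toward the current target at Speed scaled by delta seconds, without sweeping.
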(event EventBeginPlay
  (CallFunction|SetupLocations))

(event EventTick
  (params (DeltaSeconds :type Float%20%28single-precision%29))
  (CallFunction|MovetoLocations))

(fn ConstructionScript)

(fn SetupLocations
  (Variables|Locations|SetGlobalStartLocation (Transformation|GetActorLocation))
  (Variables|Locations|SetGlobalTargetLocation (Math|Transform|TransformLocation (Transformation|GetActorTransform) (Variables|Locations|GetTargetLocation)))
  (Variables|Locations|SetJourneyLength (Math|Vector|VectorLength (- (Variables|Locations|GetGlobalTargetLocation) (Variables|Locations|GetGlobalStartLocation))))
  (return))

(fn MovetoLocations
  (Utilities|FlowControl|Sequence
    (:then_0
      ;[1 1 1] Update locations
      (bind _output_get (LocalVariables|SetLocation (Transformation|GetActorLocation)))
      (LocalVariables|SetJourneyTravelled (Math|Vector|VectorLength (- _output_get (Variables|Locations|GetGlobalStartLocation)))))
    (:then_1
      ;[1 1 1] Swap direction
      (if (>= (LocalVariables|GetJourneyTravelled) (Variables|Locations|GetJourneyLength))
        (LocalVariables|SetSwap (Variables|Locations|GetGlobalStartLocation))
        (Variables|Locations|SetGlobalStartLocation (Variables|Locations|GetGlobalTargetLocation))
        (Variables|Locations|SetGlobalTargetLocation (LocalVariables|GetSwap))))
    (:then_2
      ;[1 1 1] Move
      (LocalVariables|SetDirection (Math|Vector|Normalize (- (Variables|Locations|GetGlobalTargetLocation) (Variables|Locations|GetGlobalStartLocation)) 0.001))
      (Transformation|SetActorLocation (+ (Transformation|GetActorLocation) (* (LocalVariables|GetDirection) (* (Variables|Default|GetSpeed) (Utilities|Time|GetWorldDeltaSeconds)))) false false))))